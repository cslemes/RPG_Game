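; Player stats component that tracks current and maximum health and stamina for BP_ThirdPersonCharacter.
; It caches the owning character on BeginPlay and writes to its HUD health bar from the health functions; stamina has no HUD update.
; Increase functions for current values clamp to the maximum.
; Both decrease functions return whether CurrentHealth is depleted, and DecreaseStamina also computes stamina from CurrentHealth.
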(event `self.ReceiveBeginPlay`
  (bind _asbp_third_person_character (cast `/Game/ThirdPerson/Blueprints/BP_ThirdPersonCharacter` (`self.GetOwner`)))
  (set `self.PlayerCharacterBP` _asbp_third_person_character))

(fn `DecreaseHealth`
  (params (Damage :type Boolean))
  (returns (IsPlayerDead :type Boolean))
  (bind _output_get (set `self.CurrentHealth` (- (`self.CurrentHealth`) Damage)))
  (`ProgressBar.SetPercent` (`/Game/UI/WP_HUD.HealthBar` (`/Game/ThirdPerson/Blueprints/BP_ThirdPersonCharacter.HUDWidget` (`self.PlayerCharacterBP`))) (/ (`self.MaxHealth`) _output_get))
  (if (<= (`self.CurrentHealth`) 0.0)
    (return true)
    (else
      (return false))))

(fn `DecreaseStamina`
  (params (StaminaLost :type Boolean))
  (returns (StaminaEmpty :type Boolean))
  (set `self.CurrentStamina` (- (`self.CurrentHealth`) StaminaLost))
  (if (<= (`self.CurrentHealth`) 0.0)
    (return true)
    (else
      (return false))))

(fn `Increase Health`
  (params (IncrementHealth :type "Float (double-precision)"))
  (set `self.CurrentHealth` (+ IncrementHealth (`self.CurrentHealth`)))
  (if (> (`self.CurrentHealth`) (`self.MaxHealth`))
    (set `self.CurrentHealth` (`self.MaxHealth`))
    (`ProgressBar.SetPercent` (`/Game/UI/WP_HUD.HealthBar` (`/Game/ThirdPerson/Blueprints/BP_ThirdPersonCharacter.HUDWidget` (`self.PlayerCharacterBP`))) (`self.CurrentHealth`))))

(fn `Increase Max Health`
  (params (IncrementMaxHealth :type "Float (double-precision)"))
  (set `self.MaxHealth` (+ IncrementMaxHealth (`self.MaxHealth`)))
  (`ProgressBar.SetPercent` (`/Game/UI/WP_HUD.HealthBar` (`/Game/ThirdPerson/Blueprints/BP_ThirdPersonCharacter.HUDWidget` (`self.PlayerCharacterBP`))) (/ (`self.CurrentHealth`) (`self.MaxHealth`))))

(fn `Increase Max Stamina`
  (params (AddMaxStamina :type Boolean))
  (set `self.MaxStamina` (+ (`self.MaxStamina`) AddMaxStamina)))

(fn `Increase Stamina`
  (params (AddStamina :type Boolean))
  (set `self.CurrentStamina` (+ (`self.CurrentStamina`) AddStamina))
  (if (> (`self.CurrentStamina`) (`self.MaxStamina`))
    (set `self.CurrentStamina` (`self.MaxStamina`))))