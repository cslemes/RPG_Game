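; Actor component that runs a four-step melee combo (sword montages plus a kick) on the owning BP_ThirdPersonCharacter's mesh.
; IA_Attack, gated by CanAttack, starts an attack or buffers the press in SaveAttack while IsAttacking.
; AttackIndex selects the DoOnce-guarded montage event, which advances the index.
; SwordAttackCombo, not called within this graph, consumes the buffered press to continue the chain or calls StopCombo to reset it.
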(event `self.ReceiveBeginPlay`
  (bind _asbp_third_person_character (cast `/Game/ThirdPerson/Blueprints/BP_ThirdPersonCharacter` (`self.GetOwner`)))
  (set `self.characterMesh` (`Character.Mesh` _asbp_third_person_character)))

(event `Attack 1`
  ;[1 1 1] Attack 1
  (`/Engine/EditorBlueprintResources/StandardMacros.DoOnce` false :!label _label
    (:`Completed`
      (`KismetSystemLibrary.Delay` 0.1)
      (`|PlayMontage` (`self.characterMesh`) "/Game/RPG_Character/Animations/SwordAttacks/Attack1_Montage.Attack1_Montage"
        (:`then`
          (set `self.attackIndex` 1)
          (goto _label :!via `Reset`))))))

(event `EnhancedInput|/Game/ThirdPerson/Input/Actions/IA_Attack`
  (params (ActionValue :type Boolean) (ElapsedSeconds :type "Float (double-precision)") (TriggeredSeconds :type "Float (double-precision)") (InputAction :type "InputAction Object Reference" :default "/Game/ThirdPerson/Input/Actions/IA_Attack.IA_Attack"))
  ;[1 1 1] Attack Input
  (:`Started`
    (if (`self.canAttack`)
      (`self.Sword Attack`))))

(event `Attack 2`
  ;[1 1 1] Attack 2
  (`/Engine/EditorBlueprintResources/StandardMacros.DoOnce` false :!label _label_2
    (:`Completed`
      (`KismetSystemLibrary.Delay` 0.1)
      (`|PlayMontage` (`self.characterMesh`) "/Game/RPG_Character/Animations/SwordAttacks/Attack2_Montage.Attack2_Montage"
        (:`then`
          (set `self.attackIndex` 2)
          (goto _label_2 :!via `Reset`))))))

(event `Sword Attack`
  ;[1 1 1] Sword Attack
  (if (`self.isAttacking`)
    (set `self.saveAttack` true)
    (else
      (set `self.isAttacking` true)
      (switch `int` (`self.attackIndex`) :!label _label_3
        (:`0`
          (`self.Attack 1`))
        (:`1`
          (`self.Attack 2`))
        (:`2`
          (`self.Attack 3`))
        (:`3`
          (`self.Attack 4`))))))

(event `Sword Attack Combo`
  ;[1 1 1] Combo Continue
  (if (`self.saveAttack`)
    (set `self.saveAttack` false)
    (goto _label_3)
    (else
      (`self.Stop Combo`))))

(event `Attack 3`
  ;[1 1 1] Attack 3
  (`/Engine/EditorBlueprintResources/StandardMacros.DoOnce` false :!label _label_4
    (:`Completed`
      (`KismetSystemLibrary.Delay` 0.1)
      (`|PlayMontage` (`self.characterMesh`) "/Game/RPG_Character/Animations/SwordAttacks/Kick_Montage.Kick_Montage"
        (:`then`
          (set `self.attackIndex` 3)
          (goto _label_4 :!via `Reset`))))))

(event `Stop Combo`
  ;[1 1 1] Stop Combo / Attack
  (set `self.isAttacking` false)
  (set `self.attackIndex` 0))

(event `Attack 4`
  ;[1 1 1] Attack 4
  (`/Engine/EditorBlueprintResources/StandardMacros.DoOnce` false :!label _label_5
    (:`Completed`
      (`KismetSystemLibrary.Delay` 0.1)
      (`|PlayMontage` (`self.characterMesh`) "/Game/RPG_Character/Animations/SwordAttacks/Attack3_Montage.Attack3_Montage"
        (:`then`
          (set `self.attackIndex` 4)
          (goto _label_5 :!via `Reset`))))))